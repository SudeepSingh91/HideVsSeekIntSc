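; Capturable objective actor for a Hider versus Seeker mode, picked up when a Hider touches it.
; On the server it records its start location and, on overlap while uncaptured, gives itself to a Hider not already holding one.
; HideTargetHeld then hides the Target component if the game state's LocalPlayer controls a Seeker.
; ResetPos returns the actor to its start location and clears the captured flag.
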(event OnComponentBeginOverlap(Target)
  (params (OverlappedComponent :type Primitive%20Component%20Object%20Reference) (OtherActor :type Actor%20Object%20Reference) (OtherComp :type Primitive%20Component%20Object%20Reference) (OtherBodyIndex :type Integer) (bFromSweep :type Boolean) (SweepResult :type Hit%20Result%20Structure%20%28by%20ref%29))
  ;[1 1 1] Hider Captures Target
  (Networking|SwitchHasAuthority
    (:Authority
      (bind _ashider (Utilities|Casting|CastToHider OtherActor))
      (if (not (Variables|Default|GetIsCaptured))
        (if (not (Variables|/Game/HiderBP/Blueprints/Hider.Hider_C|GetHasTarget _ashider))
          (Variables|/Game/HiderBP/Blueprints/Hider.Hider_C|SetHasTarget _ashider true)
          (Variables|/Game/HiderBP/Blueprints/Hider.Hider_C|SetTargetRef _ashider self)
          (CallFunction|HideTargetHeld))))))

(event Custom|HideTargetHeld
  ;[1 1 1] Hide Target Held
  (bind _asctpgame_state (Utilities|Casting|CastToCTPGameState (Game|GetGameState)))
  (Utilities|Casting|CastToSeeker (Pawn|GetControlledPawn (Variables|/Game/Blueprints/Daniel/CTP/CTPGameState.CTPGameState_C|GetLocalPlayer _asctpgame_state)))
  (Rendering|SetVisibility (Variables|Default|GetTarget) false false))

(event Custom|ResetPos
  ;[1 1 1] Set Position
  (Transformation|SetActorLocation (Variables|Default|GetInitPos) false false)
  (Variables|Default|SetIsCaptured false))

(event Collision|EventActorBeginOverlap
  (params (OtherActor :type Actor%20Object%20Reference)))

(event EventBeginPlay
  ;[1 1 1] Set Position
  (Networking|SwitchHasAuthority
    (:Authority
      (Variables|Default|SetInitPos (Transformation|GetActorLocation)))))

(fn ConstructionScript)