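; Practice Hider actor that starts disguised as a random prop mesh and switches to a goo mesh via ChangetoHider, losing health each call.
; As goo it drifts along a random planar vector rerolled every second.
; At zero health it flashes, spawning trails and doubling rerolled speeds, then stuns to a halt after a delay.
; An authority-only Paint event briefly spawns floor paint each tick; RemovePaint destroys all paint actors.
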(event Custom|Change%20to%20Hider
  (Components|StaticMesh|SetStaticMesh (Variables|Default|GetStaticMesh) "/Game/Geometry/FinalArt/VeetexAnim/goo_minR.goo_minR")
  (bind _output_get (Variables|Default|SetHealth (- (Variables|Default|GetHealth) 1)))
  (if (<= _output_get 0)
    (if (not (Variables|Default|GetIsFlash))
      (Variables|Default|SetIsFlash true)
      (Utilities|FlowControl|Delay 5.0)
      (Variables|Default|SetIsStun true))))

(event Custom|SetVec
  (Variables|Default|SetDelVec (Math|Vector|MakeVector (Math|Random|RandomFloatinRange -2.0 2.0) (Math|Random|RandomFloatinRange -2.0 2.0) 0.0))
  (if (Variables|Default|GetIsFlash)
    (Variables|Default|SetDelVec (* (Variables|Default|GetDelVec) 2))))

(event Custom|Paint
  (Networking|SwitchHasAuthority
    (:Authority
      (Variables|Default|SetIsPaint true)
      (Utilities|FlowControl|Delay 5.0)
      (Variables|Default|SetIsPaint false)
      (Utilities|FlowControl|Delay 0.2))))

(event Custom|RemovePaint
  (bind _outactors (Actor|GetAllActorsOfClass "/Game/Blueprints/Sudeep/Paint.Paint_C"))
  (for _array_element _outactors
    (Actor|DestroyActor _array_element)))

(event Custom|PaintTheFloor
  (Game|SpawnActorfromClass "/Game/Blueprints/Sudeep/Paint.Paint_C" (Math|Transform|MakeTransform (- (Transformation|GetActorLocation) "0,0.000000,95.000000") "0, 0, 0" "0.500000,0.500000,0.100000") "AlwaysSpawn" 0 0))

(event EventBeginPlay
  (Components|StaticMesh|SetStaticMesh (Variables|Default|GetStaticMesh) (Utilities|Array|Get(acopy) (Variables|Default|GetObjArr) (Math|Random|RandomIntegerinRange 0 (- (Utilities|Array|Length (Variables|Default|GetObjArr)) 1))))
  (Utilities|Time|SetTimerbyFunctionName 0 "SetVec" 1.0 true))

(event Collision|EventActorBeginOverlap
  (params (OtherActor :type Actor%20Object%20Reference)))

(event EventTick
  (params (DeltaSeconds :type Float%20%28single-precision%29))
  (Utilities|FlowControl|Sequence
    (:then_0
      (if (not (Variables|Default|GetIsStun))
        (if (== (Variables|/Script/Engine.StaticMeshComponent|GetStaticMesh (Variables|Default|GetStaticMesh)) "/Game/Geometry/FinalArt/VeetexAnim/goo_minR.goo_minR")
          (Transformation|AddWorldOffset (Variables|Default|GetDefaultSceneRoot1) (Variables|Default|GetDelVec) false false)
          (if (Variables|Default|GetIsFlash)
            (Game|SpawnActorfromClass "/Game/Blueprints/Sudeep/FlashTrail.FlashTrail_C" (Math|Transform|MakeTransform (+ (Transformation|GetActorLocation) "0, 0,35.000000") "0, 0, 0" "1.000000,1.000000,1.000000") "AlwaysSpawn" 0 0)))))
    (:then_1
      (if (Variables|Default|GetIsPaint)
        (CallFunction|PainttheFloor)))))

(fn ConstructionScript)