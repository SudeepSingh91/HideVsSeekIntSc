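; Game instance for Hide N Seek that manages multiplayer sessions, level travel, shared settings and gamepad menu navigation.
; Hosting creates a session, saves room info to a slot named after the player controller, then opens the map as a listen server.
; LAN searches cache non-full sessions for joining and availability checks.
; Left-stick input walks a directional graph of widget nodes after a delay, recoloring buttons and sliders to show focus.
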(event Custom|Instance_JoinLobby
  (params (PlayerController :type Player%20Controller%20Object%20Reference) (Session :type Blueprint%20Session%20Result%20Structure))
  ;[1 1 1] Comment
  (|JoinSession PlayerController Session
    (:OnSuccess
      (Development|PrintString "Joining"))
    (:OnFailure
      (Development|PrintString "Failed to Join Session"))))

(event Custom|OpenTutorial
  (params (Level :type Name))
  ;[1 1 1] Open Tutorial Level
  (Game|OpenLevel(byName) Level true "listen"))

(event Custom|CheckServerState
  (params (Controller :type Player%20Controller%20Object%20Reference) (CurServer :type Blueprint%20Session%20Result%20Structure))
  (bind _availablesessions (Variables|Default|GetAvailableSessions))
  (Variables|Default|SetavailableSessionLength 0)
  (Variables|Default|SetroomIsNotFull false)
  (Utilities|Array|Clear (Variables|Default|GetAvailableSessions))
  (bind _results (|FindSessions Controller 6 true)
    (:then
      (for _array_element _results
        (if (< (Class|FindSessionsCallbackProxy|GetCurrentPlayers _array_element) (Class|FindSessionsCallbackProxy|GetMaxPlayers _array_element))
          (Utilities|Array|Add _availablesessions _array_element)
          (Variables|Default|SetroomIsNotFull (Utilities|Enum|Equal(Enum) (Class|FindSessionsCallbackProxy|GetServerName _array_element) (Class|FindSessionsCallbackProxy|GetServerName CurServer)))
          (Variables|Default|SetavailableSessionLength (Utilities|Array|Length _availablesessions)))))
    (:OnFailure
      (Development|PrintString "Session search failed" true true "(R=1.000000,G=0.028582,B=0.000000,A=1.000000)"))))

(event Custom|Instance_UpdateAvailableSessions
  (params (PlayerController :type Player%20Controller%20Object%20Reference))
  (bind _availablesessions (Variables|Default|GetAvailableSessions))
  ;[1 1 1] Comment
  (Variables|Default|SetavailableSessionLength 0)
  (Utilities|Array|Clear (Variables|Default|GetAvailableSessions))
  (bind _results (|FindSessions PlayerController 2 true)
    (:then
      (for _array_element _results
        (if (< (Class|FindSessionsCallbackProxy|GetCurrentPlayers _array_element) (Class|FindSessionsCallbackProxy|GetMaxPlayers _array_element))
          (Utilities|Array|Add _availablesessions _array_element)))
      (Variables|Default|SetavailableSessionLength (Utilities|Array|Length _availablesessions)))
    (:OnFailure
      (Development|PrintString "Session search failed" true true "(R=1.000000,G=0.028582,B=0.000000,A=1.000000)"))))

(event Custom|OpenLobby
  ;[1 1 1] Open Lobby Level
  (Game|OpenLevel(byName) "Lobby" true "listen"))

(event Custom|NotifyInfo
  (params (InfoToNotify :type Text))
  ;[1 1 1] Info to be notified
  (Variables|Default|SetInfoNotify InfoToNotify))

(event Custom|Instance_HostLobby
  (params (GameMap :type String) (useLan :type Boolean) (RoomName :type Text) (RoomPassword :type Text) (GameMode :type String) (PlayerController :type Player%20Controller%20Object%20Reference))
  (bind _returnvalue (Utilities|GetDisplayName PlayerController))
  ;[1 1 1] Comment
  (|Session PlayerController 2 useLan
    (:OnSuccess
      (Development|PrintString _returnvalue true true "(R=0.000000,G=0.660000,B=1.000000,A=1.000000)" 1e+01)
      (bind _returnvalue_2 (SaveGame|CreateSaveGameObject "/Game/UI/MainMenu/SaveSessionInfo.SaveSessionInfo_C"))
      (bind _output_get (Variables|Default|SetSaveSessionInfoSubClass _returnvalue_2))
      (bind _assave_session_info (Utilities|Casting|CastToSaveSessionInfo _output_get))
      (Variables|/Game/UI/MainMenu/SaveSessionInfo.SaveSessionInfo_C|SetRoomName _assave_session_info RoomName)
      (Variables|/Game/UI/MainMenu/SaveSessionInfo.SaveSessionInfo_C|SetRoomPassword _assave_session_info RoomPassword)
      (Variables|/Game/UI/MainMenu/SaveSessionInfo.SaveSessionInfo_C|SetGameMode _assave_session_info GameMode)
      (Variables|/Game/UI/MainMenu/SaveSessionInfo.SaveSessionInfo_C|SetGameMap _assave_session_info GameMap)
      (SaveGame|SaveGametoSlot _output_get _returnvalue)
      (Game|OpenLevel(byName) (Utilities|String|StringToName GameMap) true "listen"))
    (:OnFailure
      (Development|PrintString "fail to create session" true true "(R=1.000000,G=0.043975,B=0.000000,A=1.000000)" 1e+01))))

(event Custom|Settings
  (params (music :type Float%20%28single-precision%29) (audio :type Float%20%28single-precision%29) (mouse :type Float%20%28single-precision%29))
  ;[1 1 1] Settings
  (Variables|Default|SetmusicVolume music)
  (Variables|Default|SetaudioVolume audio)
  (Variables|Default|SetmouseSensitive mouse))

(event Custom|TstFunction)

(event Custom|UpdateController
  (bind _returnvalue (Game|GetPlayerController 0))
  (bind _delayduration (Variables|Default|GetdelayDuration))
  (bind (_stickx _sticky) (Class|PlayerController|GetInputAnalogStickState _returnvalue "CAS_LeftStick"))
  ;[1 1 1] Controller
  (Utilities|FlowControl|Sequence
    (:then_0
      (if (> _sticky 0.7)
        (Utilities|FlowControl|Delay _delayduration)
        (bind _output_get (Variables|Default|SetbuttonIndex (.up (Utilities|Struct|BreakWidgetNode (Utilities|Array|Get(acopy) (Variables|Default|GetwidgetNodes) (Variables|Default|GetbuttonIndex))))))
        (Development|PrintString (Utilities|String|ToString(Integer) _output_get))
        (CallFunction|HighlightButton (Variables|Default|GetbuttonIndex) :!label _label)))
    (:then_1
      (if (< _sticky -0.7)
        (Utilities|FlowControl|Delay _delayduration)
        (bind _output_get_2 (Variables|Default|SetbuttonIndex (.down (Utilities|Struct|BreakWidgetNode (Utilities|Array|Get(acopy) (Variables|Default|GetwidgetNodes) (Variables|Default|GetbuttonIndex))))))
        (Development|PrintString (Utilities|String|ToString(Integer) _output_get_2))
        (goto _label)))
    (:then_2
      (if (> _stickx 0.7)
        (Utilities|FlowControl|Delay _delayduration)
        (bind _output_get_3 (Variables|Default|SetbuttonIndex (.right (Utilities|Struct|BreakWidgetNode (Utilities|Array|Get(acopy) (Variables|Default|GetwidgetNodes) (Variables|Default|GetbuttonIndex))))))
        (Development|PrintString (Utilities|String|ToString(Integer) _output_get_3))
        (goto _label)))
    (:then_3
      (if (< _stickx -0.7)
        (Utilities|FlowControl|Delay _delayduration)
        (bind _output_get_4 (Variables|Default|SetbuttonIndex (.left (Utilities|Struct|BreakWidgetNode (Utilities|Array|Get(acopy) (Variables|Default|GetwidgetNodes) (Variables|Default|GetbuttonIndex))))))
        (Development|PrintString (Utilities|String|ToString(Integer) _output_get_4))
        (goto _label)))))

(event Custom|ClearSessionList
  (Utilities|Array|Clear (Variables|Default|GetAvailableSessions)))

(fn CheckifPlayable
  (params (Server :type Blueprint%20Session%20Result%20Structure))
  (bind _availablesessions (Variables|Default|GetAvailableSessions))
  (bind _returnvalue (Utilities|Array|FindItem _availablesessions Server))
  (bind _item (Utilities|Array|Get(acopy) _availablesessions _returnvalue))
  (if (Utilities|Array|ContainsItem _availablesessions Server)
    (if (< (Class|FindSessionsCallbackProxy|GetCurrentPlayers _item) (Class|FindSessionsCallbackProxy|GetMaxPlayers _item))
      (Development|PrintString "yes" true true "(R=0.000000,G=0.660000,B=1.000000,A=1.000000)" 1e+01)
      (return true)
      (else
        _)))
  (Development|PrintString "no" true true "(R=0.000000,G=0.660000,B=1.000000,A=1.000000)" 1e+01)
  (return false))

(fn SetWidgetNodes
  (params (i_widgetNodes :type Array%20of%20Widget%20Node%20Structures) (i_defaultButtonIndex :type Integer))
  (Variables|Default|SetwidgetNodes i_widgetNodes)
  (bind _output_get (Variables|Default|SetbuttonIndex i_defaultButtonIndex))
  (CallFunction|HighlightButton _output_get))

(fn SetStick
  (params (i_stickX :type Float%20%28single-precision%29) (i_stickY :type Float%20%28single-precision%29))
  (Variables|Default|SetstickX i_stickX)
  (Variables|Default|SetstickY i_stickY))

(fn HighlightButton
  (params (i_buttonIndex :type Integer))
  (Variables|Default|SetbuttonIndex i_buttonIndex)
  (switch Utilities|FlowControl|Switch|SwitchonWidgetType (.Type (Utilities|Struct|BreakWidgetNode (Utilities|Array|Get(acopy) (Variables|Default|GetWidgetNodes) (Variables|Default|GetbuttonIndex))))
    (:NewEnumerator0
      (bind _asbutton (Utilities|Casting|CastToButton (.Widget (Utilities|Struct|BreakWidgetNode (Utilities|Array|Get(acopy) (Variables|Default|GetWidgetNodes) (Variables|Default|GetbuttonIndex)))))
        (:then
          _)
        (:CastFailed
          _))
      (Class|Button|SetBackgroundColor _asbutton "(R=0.770000,G=0.585365,B=0.139816,A=1.000000)")
      (for _index (range 0 (- (Utilities|Array|Length (Variables|Default|GetWidgetNodes)) 1))
        (if (!= _index (Variables|Default|GetbuttonIndex))
          (switch Utilities|FlowControl|Switch|SwitchonWidgetType (.Type (Utilities|Struct|BreakWidgetNode (Utilities|Array|Get(acopy) (Variables|Default|GetWidgetNodes) _index)))
            (:NewEnumerator0
              (bind _asbutton_2 (Utilities|Casting|CastToButton (.Widget (Utilities|Struct|BreakWidgetNode (Utilities|Array|Get(acopy) (Variables|Default|GetWidgetNodes) _index)))))
              (Class|Button|SetBackgroundColor _asbutton_2 "(R=0.645000,G=0.645000,B=0.645000,A=1.000000)"))
            (:NewEnumerator1
              (bind _asslider (Utilities|Casting|CastToSlider (.Widget (Utilities|Struct|BreakWidgetNode (Utilities|Array|Get(acopy) (Variables|Default|GetWidgetNodes) _index)))))
              (Class|Slider|SetSliderHandleColor _asslider))))))
    (:NewEnumerator1
      (bind _asslider_2 (Utilities|Casting|CastToSlider (.Widget (Utilities|Struct|BreakWidgetNode (Utilities|Array|Get(acopy) (Variables|Default|GetWidgetNodes) (Variables|Default|GetbuttonIndex))))))
      (Class|Slider|SetSliderHandleColor _asslider_2 "(R=0.745000,G=0.084488,B=0.069665,A=1.000000)"))))